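; SpawnGrid is a Blueprint that lays out a fixed hexagonal-style grid of static mesh tiles, with no runtime logic.
; The Construction Script runs nested X and Y loops around the origin, adding an automatically attached Static Mesh Component per cell, slightly below the actor.
; Odd rows shift half a cell along X, using the absolute value of the row index modulo two so negative rows stagger correctly.
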(event EventBeginPlay)

(event Collision|EventActorBeginOverlap
  (params (OtherActor :type Actor%20Object%20Reference)))

(event EventTick
  (params (DeltaSeconds :type Float%20%28single-precision%29)))

(fn ConstructionScript
  (for _index (range -3 3) ; X-axis loop
    (for _index_2 (range -5 5) ; Y-axis loop
      (AddComponent|AddStaticMeshComponent false (Math|Transform|MakeTransform (Math|Vector|MakeVector (- (- (* _index 86.666664) 43.333332) (* (Math|Float|Absolute(Float) (Math|Conversions|ToFloat(Integer) (Math|Integer|%(Integer) _index_2 2))) 43.333332)) (+ (* _index_2 75.0) 43.333332) -1e+02))))))